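; BulletSpawner is an actor that spawns a Bullet whenever the Shoot input action is pressed.
; It enables input from the first player controller on BeginPlay and stores its own starting location, which the graph never reads.
; Each shot spawns at the player pawn's location with a small fixed world X offset, independent of the spawner's position or the pawn's facing.
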(event `self.ReceiveBeginPlay`
  (`self.EnableInput` (`GameplayStatics.GetPlayerController` 0))
  (set `self.startLocation` (`self.K2_GetActorLocation`)))

(event `InputAction|Shoot`
  (params (Key :type "Key Structure"))
  (:`Pressed`
    (`|SpawnActorFromClass` "/Game/MP2/Blueprints/PlayerCharacter/Bullet.Bullet_C" (`KismetMathLibrary.MakeTransform` (`KismetMathLibrary.MakeVector` (+ 10.0 (.x (`self.K2_GetActorLocation` (`GameplayStatics.GetPlayerPawn` 0)))) (.y (`self.K2_GetActorLocation` (`GameplayStatics.GetPlayerPawn` 0))) (.z (`self.K2_GetActorLocation` (`GameplayStatics.GetPlayerPawn` 0))))) "Undefined" "OverrideRootScale" null null)))

(fn `UserConstructionScript`)