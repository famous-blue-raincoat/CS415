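; Bullet is a projectile actor that flies in a straight line and destroys itself after a short lifespan.
; On BeginPlay it casts the first player pawn to the learning kit character and stores the follow camera's forward vector as its direction.
; Each Tick moves it along that stored direction at ForwardSpeed, scaled by delta time, using a swept world offset, with no hit handling in the graph.
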(event `self.ReceiveBeginPlay`
  (`self.SetLifeSpan` 5.0)
  (bind _asbp_learning_kit_player_character (cast `/Game/MP2/Blueprints/PlayerCharacter/BP_LearningKit_PlayerCharacter` (`GameplayStatics.GetPlayerPawn` 0)))
  (set `self.ForwardVector` (`SceneComponent.GetForwardVector` (`/Game/MP2/Blueprints/PlayerCharacter/BP_LearningKit_PlayerCharacter.FollowCamera` _asbp_learning_kit_player_character))))

(event `self.ReceiveTick`
  (params (DeltaSeconds :type "Float (single-precision)"))
  (bind (_forwardvector_x _forwardvector_y _forwardvector_z) (`KismetMathLibrary.BreakVector` (`self.ForwardVector`)))
  (bind _forwardspeed (`self.ForwardSpeed`))
  (`self.K2_AddActorWorldOffset` (`KismetMathLibrary.MakeVector` (* DeltaSeconds _forwardspeed _forwardvector_x) (* DeltaSeconds _forwardspeed _forwardvector_y) (* DeltaSeconds _forwardspeed _forwardvector_z)) true))

(fn `UserConstructionScript`)