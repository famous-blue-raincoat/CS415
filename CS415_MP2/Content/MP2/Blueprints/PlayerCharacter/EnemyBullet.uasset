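; Enemy projectile that damages the LearningKit player character on overlap.
; On BeginPlay it caches its forward vector and sets a short lifespan, then moves along that vector every Tick using a swept world offset scaled by speed and delta time.
; Capsule overlaps ignore actors tagged Enemy and apply damage only to the player character, without destroying the bullet on hit.
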(event `self.ReceiveBeginPlay`
  (`self.SetLifeSpan` 5.0)
  (set `self.ForwardVector` (`self.GetActorForwardVector`)))

(event `self.ReceiveTick`
  (params (DeltaSeconds :type "Float (single-precision)"))
  (bind (_forwardvector_x _forwardvector_y _forwardvector_z) (`KismetMathLibrary.BreakVector` (`self.ForwardVector`)))
  (bind _forwardspeed (`self.ForwardSpeed`))
  (`self.K2_AddActorWorldOffset` (`KismetMathLibrary.MakeVector` (* DeltaSeconds _forwardspeed _forwardvector_x) (* DeltaSeconds _forwardspeed _forwardvector_y) (* DeltaSeconds _forwardspeed _forwardvector_z)) true))

(event `self.Capsule.OnComponentBeginOverlap`
  (params (OverlappedComponent :type "PrimitiveComponent Object Reference") (OtherActor :type "Actor Object Reference") (OtherComp :type "PrimitiveComponent Object Reference") (OtherBodyIndex :type Integer) (bFromSweep :type Boolean) (SweepResult :type "HitResult Structure (by ref)"))
  (if (not (`self.ActorHasTag` OtherActor "Enemy"))
    (bind _asbp_learning_kit_player_character (cast `/Game/MP2/Blueprints/PlayerCharacter/BP_LearningKit_PlayerCharacter` OtherActor))
    (`GameplayStatics.ApplyDamage` _asbp_learning_kit_player_character (`self.Damage`) null self)))

(fn `UserConstructionScript`)