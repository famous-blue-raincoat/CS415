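; BP_MorterBombs is a mortar bomb projectile that falls straight down at a set speed and explodes when its body hits something.
; On spawn it sets downward velocity and sizes a radial force to match the StrikeRadius sphere.
; The explosion applies radial damage around the impact, with that sphere as inner radius and equal minimum and base damage, fires the force impulse, plays sound and particles, then destroys itself.
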(event `self.ReceiveBeginPlay`
  (set `MovementComponent.Velocity` (`KismetMathLibrary.MakeVector` 0.0 0.0 (* (`self.Speed`) -1.0)) (`self.ProjectileMovement`))
  (set `RadialForceComponent.Radius` (`SphereComponent.GetScaledSphereRadius` (`self.StrikeRadius`)) (`self.MortarForce`)))

(event `Explode`
  (bind _damage (`self.Damage`))
  (bind _returnvalue (`SceneComponent.K2_GetComponentLocation` (`self.StrikeBody`)))
  (`GameplayStatics.ApplyRadialDamageWithFalloff` :`BaseDamage` _damage :`MinimumDamage` _damage :`Origin` (`SceneComponent.K2_GetComponentLocation` (`self.StrikeBody`)) :`DamageInnerRadius` (`SphereComponent.GetScaledSphereRadius` (`self.StrikeRadius`)) :`DamageOuterRadius` 200.0 :`DamageCauser` self :`InstigatedByController` null)
  (`RadialForceComponent.FireImpulse` (`self.MortarForce`))
  (`GameplayStatics.PlaySoundAtLocation` null _returnvalue (struct) 1.0 1.0 0.0 null null null null)
  (`GameplayStatics.SpawnEmitterAtLocation` null _returnvalue (struct) (`self.Size`))
  (`self.K2_DestroyActor`))

(event `self.StrikeBody.OnComponentHit`
  (params (HitComponent :type "PrimitiveComponent Object Reference") (OtherActor :type "Actor Object Reference") (OtherComp :type "PrimitiveComponent Object Reference") (NormalImpulse :type "Vector Structure") (Hit :type "HitResult Structure (by ref)"))
  (`self.Explode`))

(fn `UserConstructionScript`)