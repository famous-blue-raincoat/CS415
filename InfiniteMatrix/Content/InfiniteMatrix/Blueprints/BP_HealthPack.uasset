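; BP_HealthPack is a health pickup actor that heals the player on overlap.
; When a BP_Player below full health overlaps it, the pack adds a fixed amount to Health, prints a message and destroys itself; at full health it only reports that.
; The added health is not clamped to the maximum.
; An overlapping BP_Projectile is destroyed along with the pack, so shots can remove pickups.
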(event `self.HealthPack.OnComponentBeginOverlap`
  (params (OverlappedComponent :type "PrimitiveComponent Object Reference") (OtherActor :type "Actor Object Reference") (OtherComp :type "PrimitiveComponent Object Reference") (OtherBodyIndex :type Integer) (bFromSweep :type Boolean) (SweepResult :type "HitResult Structure (by ref)"))
  (`|ExecutionSequence`
    (:`then_0`
      (bind _asbp_player (cast `/Game/InfiniteMatrix/Blueprints/BP_Player` OtherActor))
      (bind _health (`/Game/InfiniteMatrix/Blueprints/BP_Player.Health` _asbp_player))
      (if (< _health 1.0)
        (set `/Game/InfiniteMatrix/Blueprints/BP_Player.Health` (+ 0.2 _health) _asbp_player)
        (`KismetSystemLibrary.PrintString` " +0.2 health" true true (struct :`R` 1.0 :`B` 0.046772 :`A` 1.0))
        (`self.K2_DestroyActor`)
        (else
          (`KismetSystemLibrary.PrintString` "health is full!" true true (struct :`R` 0.879622 :`G` 0.14996 :`B` 0.417885 :`A` 1.0)))))
    (:`then_1`
      (bind _asbp_projectile (cast `/Game/InfiniteMatrix/Blueprints/BP_Projectile` OtherActor))
      (`/Game/InfiniteMatrix/Blueprints/BP_Projectile.DestoryProjectile` _asbp_projectile)
      (`self.K2_DestroyActor`))))

(fn `UserConstructionScript`)