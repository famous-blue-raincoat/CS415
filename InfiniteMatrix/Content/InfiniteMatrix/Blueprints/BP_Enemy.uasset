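; Enemy actor that damages the player on contact and can be shot down for score.
; All logic runs from the Enemy component's begin-overlap event, which casts the other actor to player or projectile.
; A player hit shows a screen-flash widget, subtracts health, destroys the enemy and triggers death and restart display at zero health.
; A projectile hit adds to its shooter's score, then destroys both projectile and enemy.
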(event `self.Enemy.OnComponentBeginOverlap`
  (params (OverlappedComponent :type "PrimitiveComponent Object Reference") (OtherActor :type "Actor Object Reference") (OtherComp :type "PrimitiveComponent Object Reference") (OtherBodyIndex :type Integer) (bFromSweep :type Boolean) (SweepResult :type "HitResult Structure (by ref)"))
  (`|ExecutionSequence`
    (:`then_0`
      (bind _asbp_player (cast `/Game/InfiniteMatrix/Blueprints/BP_Player` OtherActor))
      (`|ExecutionSequence`
        (:`then_0`
          (bind _returnvalue (`|CreateWidget` "/Game/InfiniteMatrix/Blueprints/ScreenFlash.ScreenFlash_C" (`GameplayStatics.GetPlayerController` 0)))
          (`UserWidget.AddToViewport` _returnvalue 0))
        (:`then_1`
          (bind _health (`/Game/InfiniteMatrix/Blueprints/BP_Player.Health` _asbp_player))
          (if (> _health 0.0)
            (bind _output_get (set `/Game/InfiniteMatrix/Blueprints/BP_Player.Health` (- _health 0.2) _asbp_player))
            (`KismetSystemLibrary.PrintString` "-0.2 health!")
            (`self.K2_DestroyActor`)
            (if (<= _output_get 0.0)
              (set `/Game/InfiniteMatrix/Blueprints/BP_Player.IsDead` true _asbp_player)
              (`/Game/InfiniteMatrix/Blueprints/BP_Player.DisplayRestart` _asbp_player))))))
    (:`then_1`
      (bind _asbp_projectile (cast `/Game/InfiniteMatrix/Blueprints/BP_Projectile` OtherActor))
      (bind _shooterreference (`/Game/InfiniteMatrix/Blueprints/BP_Projectile.ShooterReference` _asbp_projectile))
      (set `/Game/InfiniteMatrix/Blueprints/BP_Player.Score` (+ (`/Game/InfiniteMatrix/Blueprints/BP_Player.Score` _shooterreference) 1.0) _shooterreference)
      (`/Game/InfiniteMatrix/Blueprints/BP_Projectile.DestoryProjectile` _asbp_projectile)
      (`self.K2_DestroyActor`))))

(fn `UserConstructionScript`)